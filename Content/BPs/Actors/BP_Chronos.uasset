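; BP_Chronos is a time-of-day actor that keeps the sky in sync with a day/night cycle.
; On BeginPlay it finds the level's sky sphere, directional light and sky light, storing each only if exactly one exists and warning if none do.
; Each Tick runs the parent's Tick, then tells the sky sphere to update its sun direction; the Blueprint itself contains no time or sun-movement logic.
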(event `self.ReceiveBeginPlay`
  ;[1 1 1] Get TimeOfDay Actors
  (`|ExecutionSequence`
    (:`then_0`
      (bind _outactors (`GameplayStatics.GetAllActorsOfClass` "/Engine/EngineSky/BP_Sky_Sphere.BP_Sky_Sphere_C"))
      (bind _returnvalue (`KismetArrayLibrary.Array_Length` _outactors))
      (if (== _returnvalue 0)
        (`KismetSystemLibrary.PrintString` "WARNING: No BP_SkySphere found in level, cannot update sky for day/night cycle.")
        (elif (== _returnvalue 1)
          (set `self.BP_SkySphere` (`|GetArrayItem` _outactors)))))
    (:`then_1`
      (bind _outactors_2 (`GameplayStatics.GetAllActorsOfClass` "/Script/Engine.DirectionalLight"))
      (bind _returnvalue_2 (`KismetArrayLibrary.Array_Length` _outactors_2))
      (if (== _returnvalue_2 0)
        (`KismetSystemLibrary.PrintString` "WARNING: No DirectionalLight found in level, cannot update sky for day/night cycle.")
        (elif (== _returnvalue_2 1)
          (set `self.PrimarySunLight` (`|GetArrayItem` _outactors_2)))))
    (:`then_2`
      (bind _outactors_3 (`GameplayStatics.GetAllActorsOfClass` "/Script/Engine.SkyLight"))
      (bind _returnvalue_3 (`KismetArrayLibrary.Array_Length` _outactors_3))
      (if (== _returnvalue_3 0)
        (`KismetSystemLibrary.PrintString` "WARNING: No SkyLight found in level, cannot update sky for day/night cycle.")
        (elif (== _returnvalue_3 1)
          (set `self.SkyLightActor` (`|GetArrayItem` _outactors_3)))))))

(event `self.ReceiveTick`
  (params (DeltaSeconds :type "Float (single-precision)"))
  ;[1 1 1] Update Solar Position
  (`parent.ReceiveTick` DeltaSeconds)
  (`/Engine/EngineSky/BP_Sky_Sphere.UpdateSunDirection` (`self.BP_SkySphere`)))

(fn `UserConstructionScript`)